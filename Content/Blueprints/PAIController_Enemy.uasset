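; AI controller for enemy pawns that starts BB_Enemy and BT_Enemy on BeginPlay.
; On perception updates, the GetSide macro compares team values from the sensed actor and controlled pawn.
; Opposing actors have their stimulus printed for debugging and, if successfully sensed, are stored as SeenTarget.
; The logic to write SeenTarget's location to the TargetLocation blackboard key is disconnected, so perception never reaches the behavior tree here.
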(event OnTargetPerceptionUpdated(PerceptionComp)
  (params (Actor :type Actor%20Object%20Reference) (Stimulus :type AI%20Stimulus%20Structure))
  (Variables|Default|SetSensedActor Actor)
  (Variables|Default|SetStimulus Stimulus)
  (Utilities|GetSide
    (:Enemy
      (CallFunction|DebugPerception (Variables|Default|GetSensedActor) (Variables|Default|GetStimulus))
      (Variables|Default|SetSeenTarget (select (.bsuccessfullysensed (Variables|Default|GetStimulus)) (Variables|Default|GetSensedActor) 0)))))

(event EventBeginPlay
  (Class|AIController|UseBlackboard "/Game/Blueprints/BB_Enemy.BB_Enemy")
  (AI|RunBehaviorTree "/Game/Blueprints/BT_Enemy.BT_Enemy"))

(event EventTick
  (params (DeltaSeconds :type Float%20%28single-precision%29)))

(fn ConstructionScript)

(fn DebugPerception
  (params (SensedActor :type Object%20Object%20Reference) (Stimulus :type AI%20Stimulus%20Structure%20%28by%20ref%29))
  (bind (_age _expirationage _strength _stimuluslocation _receiverlocation _tag _bsuccessfullysensed) (Utilities|Struct|BreakAIStimulus Stimulus))
  (Development|PrintString (Utilities|String|Append "Actor = " (Utilities|GetDisplayName SensedActor)))
  (Development|PrintString (Utilities|String|Append "Age = " (Utilities|String|ToString(Float) _age)))
  (Development|PrintString (Utilities|String|Append "Expîration Age = " (Utilities|String|ToString(Float) _expirationage)))
  (Development|PrintString (Utilities|String|Append "Strength = " (Utilities|String|ToString(Float) _strength)))
  (Development|PrintString (Utilities|String|Append "Stimulus Location = " (Utilities|String|ToString(Vector) _stimuluslocation)))
  (Development|PrintString (Utilities|String|Append "Receiver Location = " (Utilities|String|ToString(Vector) _receiverlocation)))
  (Development|PrintString (Utilities|String|Append "Tag = " (Utilities|String|ToString(Name) _tag)))
  (Development|PrintString (Utilities|String|Append "Successfully sensed = " (Utilities|String|ToString(Boolean) _bsuccessfullysensed))))