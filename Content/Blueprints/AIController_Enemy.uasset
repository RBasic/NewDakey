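; AI controller for enemies that runs the BT_Enemy behavior tree on the BB_Enemy blackboard.
; Perception updates compare the sensed actor's team, fetched via GetTeamMessage, with the controller's fixed team.
; For opposing actors it prints stimulus debug details and sets SeenTarget according to whether sensing succeeded.
; Each tick, a valid SeenTarget's location is written to the TargetLocation blackboard key.
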(event OnTargetPerceptionUpdated(AIPerception)
  (params (Actor :type Actor%20Object%20Reference) (Stimulus :type AI%20Stimulus%20Structure))
  (Variables|Perception|SetSensedActor Actor)
  (Variables|Perception|SetStimulus Stimulus)
  (Utilities|GetSide
    (:Ennemy
      (CallFunction|DebugPerception (Variables|Perception|GetSensedActor) (Variables|Perception|GetStimulus) 1e+01)
      (Variables|Perception|SetSeenTarget (select (.bsuccessfullysensed (Variables|Perception|GetStimulus)) (Variables|Perception|GetSensedActor) 0)))))

(event EventBeginPlay
  (Variables|/Script/Engine.SceneComponent|SetbAbsoluteRotation (Variables|Transformation|GetRootComponent) false)
  (Class|AIController|UseBlackboard "/Game/Blueprints/BB_Enemy.BB_Enemy")
  (AI|RunBehaviorTree "/Game/Blueprints/BT_Enemy.BT_Enemy"))

(event EventTick
  (params (DeltaSeconds :type Float%20%28single-precision%29))
  (bind _seentarget (Variables|Perception|GetSeenTarget)
    (:then
      (AI|Components|Blackboard|SetValueasVector (Variables|Default|GetBlackboard) (Utilities|String|StringToName "TargetLocation") (Transformation|GetActorLocation _seentarget)))
    (:else)))

(fn ConstructionScript)

(fn DebugPerception
  (params (Object :type Object%20Object%20Reference) (Stimulus :type AI%20Stimulus%20Structure) (Duration :type Float%20%28single-precision%29))
  (bind (_age _expirationage _strength _stimuluslocation _receiverlocation _tag _bsuccessfullysensed) (Utilities|Struct|BreakAIStimulus Stimulus))
  (Development|PrintString (Utilities|String|Append "Actor = " (Utilities|GetDisplayName Object)) true true "(R=0.000000,G=0.660000,B=1.000000,A=1.000000)" Duration)
  (Development|PrintString (Utilities|String|Append "Age = " (Utilities|String|ToString(Float) _age)) true true "(R=0.000000,G=0.660000,B=1.000000,A=1.000000)" Duration)
  (Development|PrintString (Utilities|String|Append "Expîration Age = " (Utilities|String|ToString(Float) _expirationage)) true true "(R=0.000000,G=0.660000,B=1.000000,A=1.000000)" Duration)
  (Development|PrintString (Utilities|String|Append "Strength = " (Utilities|String|ToString(Float) _strength)) true true "(R=0.000000,G=0.660000,B=1.000000,A=1.000000)" Duration)
  (Development|PrintString (Utilities|String|Append "Stimulus Location = " (Utilities|String|ToString(Vector) _stimuluslocation)) true true "(R=0.000000,G=0.660000,B=1.000000,A=1.000000)" Duration)
  (Development|PrintString (Utilities|String|Append "Receiver Location = " (Utilities|String|ToString(Vector) _receiverlocation)) true true "(R=0.000000,G=0.660000,B=1.000000,A=1.000000)" Duration)
  (Development|PrintString (Utilities|String|Append "Tag = " (Utilities|String|ToString(Name) _tag)) true true "(R=0.000000,G=0.660000,B=1.000000,A=1.000000)" Duration)
  (Development|PrintString (Utilities|String|Append "Successfully sensed = " (Utilities|String|ToString(Boolean) _bsuccessfullysensed)) true true "(R=0.000000,G=0.660000,B=1.000000,A=1.000000)" Duration))

(fn GetTeam
  (return "NewEnumerator1"))