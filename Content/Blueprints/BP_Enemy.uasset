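; Enemy Blueprint that ties its AI controller to the skeletal mesh so that perception follows the head.
; On BeginPlay the controller's root component snaps to the mesh's PerceptionHolder socket, keeping world scale.
; The construction script also attempts an attachment of AIController_Enemy to the head socket with relative transforms.
; Taking damage only prints a debug string with the damage causer's name.
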(event Game|Damage|EventAnyDamage
  (params (Damage :type Float%20%28single-precision%29) (DamageType :type Damage%20Type%20Object%20Reference) (InstigatedBy :type Controller%20Object%20Reference) (DamageCauser :type Actor%20Object%20Reference))
  (Development|PrintString (Utilities|String|Append (Utilities|GetDisplayName DamageCauser) " mafé bobo")))

(event EventBeginPlay
  (Transformation|AttachComponentToComponent (Variables|/Script/Engine.Actor|GetRootComponent (Pawn|GetController)) (Variables|Character|GetMesh) "PerceptionHolder" "SnapToTarget" "SnapToTarget" "KeepWorld" true) ; Attach perception to head bone
)

(fn ConstructionScript
  (Transformation|AttachComponentToComponent (.AsAIController%20Enemy (Utilities|Casting|CastToAIController_Enemy (Pawn|GetController))) (Variables|Character|GetMesh) "head" "KeepRelative" "KeepRelative" "KeepRelative" true))